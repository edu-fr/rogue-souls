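; Gameplay ability that dashes the avatar in its last movement input direction, or forward when there is no input.
; On activation it applies a short constant root motion force and adds the Dash gameplay cue, which is removed when the ability ends.
; When the force finishes, velocity is clamped to the pawn's movement component max speed and the ability ends.
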(event `self.K2_ActivateAbility`
  (`AbilityTask_ApplyRootMotionConstantForce.ApplyRootMotionConstantForce` "None" (`self.GetDashDirection`) 2000.0 0.3 false null "ClampVelocity" (0.0 0.0 0.0) (`self.GetMaxSpeed`)
    (:`then`
      (`self.K2_AddGameplayCue` (struct :`TagName` "GameplayCue.Dash")))
    (:`OnFinish`
      (`self.K2_EndAbility`))))

(fn `GetDashDirection`
  (returns (Direction :type "Vector Structure"))
  (bind _aspawn (cast `Pawn` (`self.GetAvatarActorFromActorInfo`)))
  (bind _returnvalue (`Pawn.GetLastMovementInputVector` _aspawn))
  (if (`KismetMathLibrary.Vector_IsZero` _returnvalue)
    ; Return forward if not pawn or not input
    (return (`Actor.GetActorForwardVector` (`self.GetAvatarActorFromActorInfo`)))
    (else
      ; Return input dir as expected
      (return _returnvalue))))

(fn `GetMaxSpeed`
  (returns (MaxSpeed :type "Float (double-precision)"))
  (bind _aspawn (cast `Pawn` (`self.GetAvatarActorFromActorInfo`))
    (:`then`
      (return (`MovementComponent.GetMaxSpeed` (`Pawn.GetMovementComponent` _aspawn))))
    (:`CastFailed`
      ; If not pawn return 0
      (return 0.0))))